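; Custom game state that runs an optional time-of-day clock and animates cable wires in the level.
; On BeginPlay it caches all CableActors and the sun sky, enabling real-time skylight capture and a looping timer when time elapse is on.
; The timer advances a seconds-in-day counter into the sky's time, resetting at midnight; IsBetweenTime checks its hour.
; Every Tick randomly scales each cable's force to fake waving.
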(event Custom|TimeTick
  (bind _sunsky (Variables|Default|GetSunSky))
  (if (>= (+ (Variables|Default|GetTimeSecondsInDay) (Variables|Default|GetTimeTickAddSeconds)) 86400)
    (Variables|Default|SetTimeSecondsInDay 0)
    (else
      (Variables|Default|SetTimeSecondsInDay (+ (Variables|Default|GetTimeSecondsInDay) (Variables|Default|GetTimeTickAddSeconds)))))
  (Variables|/Game/Blueprints/BP_CustomSunSky1.BP_CustomSunSky1_C|SetHours _sunsky (.Hours (Class|KismetMathLibrary|BreakTimespan2 (Math|Timespan|MakeTimespan 0 0 0 (Variables|Default|GetTimeSecondsInDay)))))
  (Variables|/Game/Blueprints/BP_CustomSunSky1.BP_CustomSunSky1_C|SetMinutes _sunsky (.Minutes (Class|KismetMathLibrary|BreakTimespan2 (Math|Timespan|MakeTimespan 0 0 0 (Variables|Default|GetTimeSecondsInDay)))))
  (Variables|/Game/Blueprints/BP_CustomSunSky1.BP_CustomSunSky1_C|SetSeconds _sunsky (.Seconds (Class|KismetMathLibrary|BreakTimespan2 (Math|Timespan|MakeTimespan 0 0 0 (Variables|Default|GetTimeSecondsInDay))))))

(event EventBeginPlay
  (bind _enabletimeelapse (Variables|Default|GetEnableTimeElapse))
  (bind _outactors (Actor|GetAllActorsOfClass "/Script/CableComponent.CableActor"))
  (Variables|Default|SetWires _outactors)
  (bind _returnvalue (Actor|GetActorOfClass "/Game/Blueprints/BP_CustomSunSky1.BP_CustomSunSky1_C"))
  (bind _output_get (Variables|Default|SetSunSky _returnvalue))
  (Variables|Default|SetSunSkyLight (Actor|GetComponentbyClass _output_get "/Script/Engine.SkyLightComponent"))
  (Class|SkyLightComponent|SetRealTimeCapture (Variables|Default|GetSunSkyLight) _enabletimeelapse)
  (if _enabletimeelapse
    (Variables|Default|SetTimeSecondsInDay (Math|Float|Truncate (Math|Timespan|GetTotalSeconds (Class|KismetMathLibrary|MakeTimespan2 0 (Variables|/Game/Blueprints/BP_CustomSunSky1.BP_CustomSunSky1_C|GetHours (Variables|Default|GetSunSky)) (Variables|/Game/Blueprints/BP_CustomSunSky1.BP_CustomSunSky1_C|GetMinutes (Variables|Default|GetSunSky)) (Variables|/Game/Blueprints/BP_CustomSunSky1.BP_CustomSunSky1_C|GetSeconds (Variables|Default|GetSunSky))))))
    (Utilities|Time|SetTimerbyEvent (delegate Custom|TimeTick) (/ 1.0 (Variables|Default|GetTimerTickAmoutInSecond)) true true)))

(event EventTick
  (params (DeltaSeconds :type Float%20%28single-precision%29))
  (CallFunction|WaveAllWires))

(fn ConstructionScript)

(fn IsBetweenTime
  (params (FirstHour :type Integer) (SecondHour :type Integer))
  (bind _timesecondsinday (Variables|Default|GetTimeSecondsInDay))
  (bind _returnvalue (Math|Timespan|MakeTimespan 0 0 0 _timesecondsinday))
  (bind _hours (Class|KismetMathLibrary|BreakTimespan2 _returnvalue))
  (return (and (< FirstHour _hours) (> SecondHour _hours))))

(fn WaveAllWires
  (for _array_element (Variables|Default|GetWires)
    (Variables|/Script/CableComponent.CableComponent|SetCableForce (Variables|/Script/CableComponent.CableActor|GetCableComponent _array_element) (* (Variables|Default|GetWireWaveForce) (Math|Random|RandomFloat)))))