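; BP_Door is a password-locked door that swings open on a correct code and closes when an overlap with its box ends.
; Beginning an overlap turns on the BPCPasswordLock component, whose correct-password callback sets the open target angle.
; Ending an overlap resets that angle to closed, without switching the lock off.
; Tick rotates the door's yaw toward the target at constant speed via RInterpToConstant until it matches within a small tolerance.
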(event OnComponentBeginOverlap(Box)
  (params (OverlappedComponent :type Primitive%20Component%20Object%20Reference) (OtherActor :type Actor%20Object%20Reference) (OtherComp :type Primitive%20Component%20Object%20Reference) (OtherBodyIndex :type Integer) (bFromSweep :type Boolean) (SweepResult :type Hit%20Result%20Structure%20%28by%20ref%29))
  (Class|PasswordLockComponent|TurnonorOff (Variables|Default|GetBPC_PasswordLock) true))

(event OnComponentEndOverlap(Box)
  (params (OverlappedComponent :type Primitive%20Component%20Object%20Reference) (OtherActor :type Actor%20Object%20Reference) (OtherComp :type Primitive%20Component%20Object%20Reference) (OtherBodyIndex :type Integer))
  (Variables|Default|SetDoorOpenAngle 0.0))

(event Custom|OnPasswordCorrect
  (Variables|Default|SetDoorOpenAngle -9e+01))

(event EventBeginPlay
  (EventDispatchers|BindEventtoOnPasswordCorrected (Variables|Default|GetBPC_PasswordLock) (delegate Custom|OnPasswordCorrect)))

(event Collision|EventActorBeginOverlap
  (params (OtherActor :type Actor%20Object%20Reference)))

(event EventTick
  (params (DeltaSeconds :type Float%20%28single-precision%29))
  (bind _door (Variables|Default|GetDoor))
  (bind _relativerotation (Variables|/Script/Engine.SceneComponent|GetRelativeRotation _door))
  (if (CallFunction|NeedDoAnim _relativerotation)
    (CallFunction|DoAnimation _relativerotation DeltaSeconds)))

(fn ConstructionScript)

(fn NeedDoAnim
  (params (CurRotator :type Rotator%20%28by%20ref%29))
  (return (Utilities|Operators|NotEqual(!=) (.Z (Math|Rotator|GetAxes CurRotator)) (Variables|Default|GetDoorOpenAngle) 0.0001)))

(fn DoAnimation
  (params (CurRotator :type Rotator%20%28by%20ref%29) (DeltaTime :type Float%20%28double-precision%29))
  (Transformation|SetRelativeRotation (Variables|Default|GetDoor) (Class|KismetMathLibrary|RInterptoConstant CurRotator (Math|Rotator|MakeRotator 0.0 0.0 (Variables|Default|GetDoorOpenAngle)) DeltaTime 9e+01) false false))