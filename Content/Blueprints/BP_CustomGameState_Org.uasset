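; Game state Blueprint that runs an optional day/night clock, driving the sun and sky and switching night lights.
; On BeginPlay it seeds seconds-in-day from BP_CustomSunSky and starts a looping timer.
; Each tick advances and wraps the time, writes it back to the sky, then uses an hour-range check to toggle one SpotLight and all BP_NeonLight actors, re-querying the neon lights every tick.
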(event Custom|TimeTick
  (bind _result (CallFunction|IsBetweenTime 7 20))
  (bind _sunsky (Variables|Default|GetSunSky))
  (bind _returnvalue (not _result))
  (if (>= (+ (Variables|Default|GetTimeSecondsInDay) (Variables|Default|GetTimeTickAddSeconds)) 86400)
    (Variables|Default|SetTimeSecondsInDay 0)
    (else
      (Variables|Default|SetTimeSecondsInDay (+ (Variables|Default|GetTimeSecondsInDay) (Variables|Default|GetTimeTickAddSeconds)))))
  (Variables|/Game/Blueprints/BP_CustomSunSky.BP_CustomSunSky_C|SetHours _sunsky (.Hours (Class|KismetMathLibrary|BreakTimespan2 (Math|Timespan|MakeTimespan 0 0 0 (Variables|Default|GetTimeSecondsInDay)))))
  (Variables|/Game/Blueprints/BP_CustomSunSky.BP_CustomSunSky_C|SetMinutes _sunsky (.Minutes (Class|KismetMathLibrary|BreakTimespan2 (Math|Timespan|MakeTimespan 0 0 0 (Variables|Default|GetTimeSecondsInDay)))))
  (Variables|/Game/Blueprints/BP_CustomSunSky.BP_CustomSunSky_C|SetSeconds _sunsky (.Seconds (Class|KismetMathLibrary|BreakTimespan2 (Math|Timespan|MakeTimespan 0 0 0 (Variables|Default|GetTimeSecondsInDay)))))
  (Rendering|SetVisibility (Variables|/Script/Engine.SpotLight|GetSpotLightComponent (Variables|Default|GetSpotLight)) _returnvalue false)
  (bind _outactors (Actor|GetAllActorsOfClass "/Game/Blueprints/BP_NeonLight.BP_NeonLight_C"))
  (for _array_element _outactors
    (Class|NeonLightActor|Turnon _array_element _returnvalue)))

(event EventBeginPlay
  (if (Variables|Default|GetEnableTimeElapse)
    (bind _returnvalue (Actor|GetActorOfClass "/Game/Blueprints/BP_CustomSunSky.BP_CustomSunSky_C"))
    (bind _output_get (Variables|Default|SetSunSky _returnvalue))
    (Variables|Default|SetTimeSecondsInDay (Math|Float|Truncate (Math|Timespan|GetTotalSeconds (Class|KismetMathLibrary|MakeTimespan2 0 (Variables|/Game/Blueprints/BP_CustomSunSky.BP_CustomSunSky_C|GetHours _output_get) (Variables|/Game/Blueprints/BP_CustomSunSky.BP_CustomSunSky_C|GetMinutes _output_get) (Variables|/Game/Blueprints/BP_CustomSunSky.BP_CustomSunSky_C|GetSeconds _output_get)))))
    (Utilities|Time|SetTimerbyEvent (delegate Custom|TimeTick) (/ 1.0 (Variables|Default|GetTimerTickAmoutInSecond)) true true)
    (bind _returnvalue_2 (Actor|GetActorOfClass "/Script/Engine.SpotLight"))
    (Variables|Default|SetSpotLight _returnvalue_2)))

(fn ConstructionScript)

(fn IsBetweenTime
  (params (FirstHour :type Integer) (SecondHour :type Integer))
  (bind _timesecondsinday (Variables|Default|GetTimeSecondsInDay))
  (bind _returnvalue (Math|Timespan|MakeTimespan 0 0 0 _timesecondsinday))
  (bind _hours (Class|KismetMathLibrary|BreakTimespan2 _returnvalue))
  (return (and (< FirstHour _hours) (> SecondHour _hours))))